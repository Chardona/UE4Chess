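; Queen chess piece Blueprint that shows the squares it can move to.
; ShowPossibleMoves clears existing highlights through the game mode, then runs diagonal, horizontal and vertical highlight helpers with the piece's color, and returns false.
; Those helpers are not defined here, and the event graph holds only disabled stub events.
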(event EventBeginPlay
  (|CallParentFunction) ; This node is disabled and will not be called.\nDrag off pins to build functionality.
)

(event Collision|EventActorBeginOverlap
  (params (OtherActor :type Actor%20Object%20Reference))
  (|CallParentFunction OtherActor) ; This node is disabled and will not be called.\nDrag off pins to build functionality.
)

(event EventTick
  (params (DeltaSeconds :type Float%20%28single-precision%29))
  (|CallParentFunction DeltaSeconds) ; This node is disabled and will not be called.\nDrag off pins to build functionality.
)

(fn ConstructionScript
  (|CallParentFunction))

(fn ShowPossibleMoves
  (bind _color (Variables|Default|GetColor))
  (Utilities|FlowControl|Sequence
    (:then_0
      (Default|UnhighlightSquares (Variables|Default|GetGameModeRef)))
    (:then_1
      (CallFunction|HighlightDiagonalSquares (Variables|Default|GetColor)))
    (:then_2
      (CallFunction|HighlightHorizontalSquares _color))
    (:then_3
      (CallFunction|HighlightVerticalSquares _color))
    (:then_4
      (return false))))