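; BP_Pawn is the chess pawn piece, highlighting its possible moves on the board.
; ShowPossibleMoves derives direction from the active player's color, clears old highlights, then marks forward, initial double-step and diagonal capture squares through GameMode occupancy queries.
; En passant uses piece and player move counts to qualify an adjacent enemy pawn, checking only the Y+1 side.
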(event EventBeginPlay)

(event Collision|EventActorBeginOverlap
  (params (OtherActor :type Actor%20Object%20Reference)))

(event EventTick
  (params (DeltaSeconds :type Float%20%28single-precision%29)))

(fn ConstructionScript
  (|CallParentFunction))

(fn HighlightPawnSquare
  (params (X :type Integer) (Y :type Integer))
  (Default|HighlightSquare (Variables|Default|GetGameModeRef) X Y))

(fn SetDirectionValue
  (switch Utilities|FlowControl|Switch|SwitchonEN_Color (Default|GetActivePlayerColor (Variables|Default|GetGameModeRef))
    (:NewEnumerator0
      (Variables|setup|SetDirectionValue (Variables|setup|GetWhiteDirection)))
    (:NewEnumerator1
      (Variables|setup|SetDirectionValue (Variables|setup|GetBlackDirection)))))

(fn SetFirstSquare
  (bind _directionvalue (Variables|setup|GetDirectionValue))
  (bind _x (Variables|Default|GetX))
  (bind _y (Variables|Default|GetY))
  (bind _returnvalue (+ _x _directionvalue))
  (if (.IsOccupied (Default|GetOccupant (Variables|Default|GetGameModeRef) _returnvalue _y (Variables|Default|GetColor)))
    (return false)
    (else
      (Gameplay|HighlightPawnSquare _returnvalue _y)
      (return true))))

(fn SetSecondSquare
  (bind _directionvalue (Variables|setup|GetDirectionValue))
  (bind _x (Variables|Default|GetX))
  (bind _y (Variables|Default|GetY))
  (bind _returnvalue (* _directionvalue 2))
  (bind _returnvalue_2 (+ _x _returnvalue))
  (if (and (Variables|Default|GetIsInitialMove) (not (.IsOccupied (Default|GetOccupant (Variables|Default|GetGameModeRef) _returnvalue_2 _y (Variables|Default|GetColor)))))
    (Gameplay|HighlightPawnSquare _returnvalue_2 _y)))

(fn SetAttackSquareRight
  (bind _gamemoderef (Variables|Default|GetGameModeRef))
  (bind _x (Variables|Default|GetX))
  (bind _color (Variables|Default|GetColor))
  (bind _y (Variables|Default|GetY))
  (bind _directionvalue (Variables|setup|GetDirectionValue))
  (bind _returnvalue (+ _x _directionvalue))
  (bind _returnvalue_2 (+ _y 1))
  (bind (_chesspiece _isoccupied _isoccupiedbyfriend_) (Default|GetOccupant _gamemoderef _returnvalue _returnvalue_2 _color))
  (if (and _isoccupied (not _isoccupiedbyfriend_))
    (Gameplay|HighlightPawnSquare _returnvalue _returnvalue_2)))

(fn SetAttackSquareLeft
  (bind _gamemoderef (Variables|Default|GetGameModeRef))
  (bind _x (Variables|Default|GetX))
  (bind _color (Variables|Default|GetColor))
  (bind _y (Variables|Default|GetY))
  (bind _directionvalue (Variables|setup|GetDirectionValue))
  (bind _returnvalue (- _y 1))
  (bind _returnvalue_2 (+ _x _directionvalue))
  (bind (_chesspiece _isoccupied _isoccupiedbyfriend_) (Default|GetOccupant _gamemoderef _returnvalue_2 _returnvalue _color))
  (if (and _isoccupied (not _isoccupiedbyfriend_))
    (Gameplay|HighlightPawnSquare _returnvalue_2 _returnvalue)))

(fn IsEnPassantCandidate
  (params (OpponentPawn :type BP%20Chess%20Piece%20Object%20Reference))
  (bind _gamemoderef (Variables|Default|GetGameModeRef))
  (return (and (== (Variables|/Game/Chess/Blueprints/ChessPieces/BP_ChessPiece.BP_ChessPiece_C|GetChessPieceMoveCount OpponentPawn) 1) (or (== (Variables|/Game/Chess/Blueprints/ChessPieces/BP_ChessPiece.BP_ChessPiece_C|GetPlayerMoveCount OpponentPawn) (Default|GetActivePlayerMoveCount _gamemoderef)) (== (+ (Variables|/Game/Chess/Blueprints/ChessPieces/BP_ChessPiece.BP_ChessPiece_C|GetPlayerMoveCount OpponentPawn) 1) (Default|GetActivePlayerMoveCount _gamemoderef))))))

(fn SetEnPassantSquare
  (bind _gamemoderef (Variables|Default|GetGameModeRef))
  (bind _x (Variables|Default|GetX))
  (bind _color (Variables|Default|GetColor))
  (bind _y (Variables|Default|GetY))
  (bind _returnvalue (+ _y 1))
  (bind (_chesspiece _isoccupied _isoccupiedbyfriend_) (Default|GetOccupant _gamemoderef _x _returnvalue _color))
  (bind (_asbp_pawn _bsuccess) (Utilities|Casting|CastToBP_Pawn _chesspiece))
  (if (Math|Boolean|ANDBoolean _bsuccess _isoccupied (not _isoccupiedbyfriend_))
    (if (Gameplay|IsEnPassantCandidate _asbp_pawn)
      (Gameplay|HighlightPawnSquare (+ (Variables|Default|GetX) (Variables|setup|GetDirectionValue)) _returnvalue))))

(fn ShowPossibleMoves
  (Utilities|FlowControl|Sequence
    (:then_0
      (Gameplay|SetDirectionValue)
      (Variables|Default|SetIsEnPassant false)
      (Default|SetMessage (Variables|Default|GetPlayerControllerRef)))
    (:then_1
      (Default|UnhighlightSquares (Variables|Default|GetGameModeRef)))
    (:then_2
      (bind _success (Gameplay|SetFirstSquare))
      (if _success
        (Gameplay|SetSecondSquare)))
    (:then_3
      (Gameplay|SetAttackSquareLeft))
    (:then_4
      (Gameplay|SetAttackSquareRight))
    (:then_5
      (Gameplay|SetEnPassantSquare))
    (:then_6
      (return (Variables|Default|GetIsKing)))))